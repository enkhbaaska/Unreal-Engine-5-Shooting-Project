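; BP_SmallSphere is a short-lived moving sphere actor that follows a curving path and then winks out.
; On BeginPlay it picks a random, scaled rotation rate without roll and starts a lifetime timer.
; Each Tick moves it along its forward vector and applies that rotation, so the heading keeps changing.
; When the timer fires, a timeline drives the mesh's uniform scale, then destroys the actor.
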(event Custom|WinkOut
  (bind _scale (Timeline|WinkOutTimeline Play)
    (:Update
      (CallFunction|ScaleSphere _scale))
    (:Finished
      (Actor|DestroyActor))))

(event EventBeginPlay
  (CallFunction|InitialiseDeltaRotation)
  (Utilities|Time|SetTimerbyEvent (delegate Custom|WinkOut) (Variables|Default|GetLifetime)))

(event Collision|EventActorBeginOverlap
  (params (OtherActor :type Actor%20Object%20Reference)))

(event EventTick
  (params (DeltaSeconds :type Float%20%28single-precision%29))
  (CallFunction|UpdateLocation DeltaSeconds)
  (CallFunction|UpdateRotation DeltaSeconds))

(fn ConstructionScript)

(fn InitialiseDeltaRotation
  (Variables|SphereMovement|SetDelta%20Rotation (* (Math|Random|RandomRotator false) (Variables|SphereMovement|GetRotationScaleFactor))))

(fn UpdateLocation
  (params (DeltaSeconds :type Float%20%28double-precision%29))
  (Transformation|AddActorWorldOffset (* (Transformation|GetActorForwardVector) (* DeltaSeconds (Variables|SphereMovement|GetSpeed)))))

(fn UpdateRotation
  (params (DeltaSeconds :type Float%20%28single-precision%29))
  (Class|Actor|AddActorWorldRotation (* (Variables|SphereMovement|GetDelta%20Rotation) DeltaSeconds)))

(fn ScaleSphere
  (params (Scale :type Float%20%28single-precision%29))
  (Transformation|SetWorldScale3D (Variables|Default|GetSphereMesh) (Math|Vector|MakeVector Scale Scale Scale)))